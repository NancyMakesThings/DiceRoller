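; Player controller for the dice roller that lets the mouse pick up and throw dice.
; Pressing on a BP_Dice grabs it with a physics handle, which follows the cursor on Tick at a fixed height.
; Release adds a random angular impulse; the debug arrow and print re-roll their random values, so differ from that impulse.
; Selection events keep one actor selected, deselecting others via interface; multi-move logic is disconnected.
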(event Custom|AddActorSelectedToList
  (params (SelectedActor :type Actor%20Object%20Reference))
  ;[1 1 1] Highlight Actor
  (CallFunction|DeselectAllActors)
  (Utilities|Array|Add (Variables|Default|GetSelectedActors) SelectedActor))

(event Custom|DeselectAllActors
  ;[1 1 1] Highlight Actor
  (for _array_element (Variables|Default|GetSelectedActors)
    (if (Utilities|DoesObjectImplementInterface _array_element "/Game/DiceRoller/Core/Dice/BPI_SelectionEvents.BPI_SelectionEvents_C")
      (Class|BPISelectionEvents|DeselectThis(Message) _array_element)))
  (Utilities|Array|Clear (Variables|Default|GetSelectedActors)))

(event Input|EnhancedActionEvents|EnhancedInputActionIA_MouseSelection
  (params (ActionValue :type Vector%202D%20Structure) (ElapsedSeconds :type Float%20%28double-precision%29) (TriggeredSeconds :type Float%20%28double-precision%29) (InputAction :type Input%20Action%20Object%20Reference :default "/Game/DiceRoller/Core/Player/Input/IA_MouseSelection.IA_MouseSelection"))
  (bind _returnvalue (Math|Random|RandomFloatinRange -1.0 1.0))
  (bind _returnvalue_2 (Math|Random|RandomFloatinRange -1.0 1.0))
  (bind _hitresult (Game|Player|GetHitResultUnderCursorbyChannel "TraceTypeQuery1" true))
  (bind _returnvalue_3 (Math|Random|RandomFloatinRange -1.0 1.0))
  (bind _angularimpulsemagnitude (Variables|Default|GetAngularImpulseMagnitude))
  (bind (_bblockinghit _binitialoverlap _time _distance _location _impactpoint _normal _impactnormal _physmat _hitactor _hitcomponent) (Collision|BreakHitResult _hitresult))
  (bind _returnvalue_4 (Math|Vector|MakeVector _returnvalue _returnvalue_3 _returnvalue_2))
  (bind _returnvalue_5 (* _returnvalue_4 _angularimpulsemagnitude))
  ;[1 1 1] Grab Actor
  (:Started
    (Utilities|Casting|CastToBP_Dice _hitactor)
    (Variables|Default|SetOriginalDistanceToObject _distance)
    (Variables|Default|SetIsGrabbingComponent true)
    (bind _output_get (Variables|Default|SetGrabbedComponent _hitcomponent))
    (Physics|Components|PhysicsHandle|GrabComponentatLocationwithRotation (Variables|Default|GetPhysicsHandle) _output_get "None" (Physics|GetCenterOfMass _hitcomponent "None") "0, 0, 0"))
  (:Completed
    (if (Variables|Default|GetIsGrabbingComponent)
      (Class|PrimitiveComponent|AddAngularImpulseinDegrees (Variables|Default|GetGrabbedComponent) _returnvalue_5 "None" true)
      (Rendering|Debug|DrawDebugArrow (Transformation|GetWorldLocation (Variables|Default|GetGrabbedComponent)) (+ (Transformation|GetWorldLocation (Variables|Default|GetGrabbedComponent)) _returnvalue_5) 1e+01 "(R=1.000000,G=0.000000,B=0.000000,A=1.000000)" 2.0 1e+01)
      (Development|PrintString (Utilities|String|ToString(Vector) _returnvalue_5))
      (Variables|Default|SetGrabbedComponent 0)
      (Physics|Components|PhysicsHandle|ReleaseComponent (Variables|Default|GetPhysicsHandle))
      (Variables|Default|SetIsGrabbingComponent false))))

(event Input|EnhancedActionEvents|EnhancedInputActionIA_MouseAction
  (params (ActionValue :type Vector%202D%20Structure) (ElapsedSeconds :type Float%20%28double-precision%29) (TriggeredSeconds :type Float%20%28double-precision%29) (InputAction :type Input%20Action%20Object%20Reference :default "/Game/DiceRoller/Core/Player/Input/IA_MouseAction.IA_MouseAction"))
  ;[1 1 1] Move Multiple (not in use)
)

(event EventTick
  (params (DeltaSeconds :type Float%20%28single-precision%29))
  (bind (_worldlocation _worlddirection) (Game|Player|ConvertMouseLocationToWorldSpace))
  (bind _originaldistancetoobject (Variables|Default|GetOriginalDistanceToObject))
  (bind _returnvalue (* _worlddirection _originaldistancetoobject))
  (bind _returnvalue_2 (+ _worldlocation _returnvalue))
  ;[1 1 1] Grab Actor
  (if (Variables|Default|GetIsGrabbingComponent)
    (Physics|Components|PhysicsHandle|SetTargetLocation (Variables|Default|GetPhysicsHandle) (Math|Vector|MakeVector (.x _returnvalue_2) (.y _returnvalue_2) (Variables|Default|GetGrabLocationZ)))))

(fn ConstructionScript)