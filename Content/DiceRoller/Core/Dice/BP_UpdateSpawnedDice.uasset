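; Component on BP_Dice that reconfigures its owning die to a given dice type and the current look stored in MyGameInstance.
; UpdateSpawnedDice sets the type, then has BPDecodeDiceMesh resolve a mesh from that type and the current mesh style.
; It applies the mesh, calls RandomFall again as the mesh change requires, then sets face and number materials on the two material slots.
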(event EventBeginPlay)

(event EventTick
  (params (DeltaSeconds :type Float%20%28single-precision%29)))

(fn UpdateSpawnedDice
  (params (DiceType :type DiceType%20Enum%20%28by%20ref%29 :default "D4"))
  (bind _asbp_dice (Utilities|Casting|CastToBP_Dice (Components|GetOwner)))
  (bind _asmy_game_instance (Utilities|Casting|CastToMyGameInstance (Game|GetGameInstance)))
  (Variables|/Script/DiceRoller.Dice|SetType _asbp_dice DiceType)
  (bind _outmesh (Default|DecodeDiceMesh (Variables|/Game/DiceRoller/Core/Dice/BP_Dice.BP_Dice_C|GetBP_DecodeDiceMesh _asbp_dice) (.meshstyle (Variables|/Script/DiceRoller.MyGameInstance|GetCurrentDiceProp _asmy_game_instance)) DiceType))
  (Class|Dice|UpdateMesh _asbp_dice _outmesh)
  (Class|Dice|RandomFall _asbp_dice) ; Additional RandomFall() needed after changing mesh
  (Rendering|Material|SetMaterial (Variables|/Script/DiceRoller.Dice|GetDiceMesh _asbp_dice) 0 (.matface (Variables|/Script/DiceRoller.MyGameInstance|GetCurrentDiceProp _asmy_game_instance)))
  (Rendering|Material|SetMaterial (Variables|/Script/DiceRoller.Dice|GetDiceMesh _asbp_dice) 1 (.matnum (Variables|/Script/DiceRoller.MyGameInstance|GetCurrentDiceProp _asmy_game_instance))))