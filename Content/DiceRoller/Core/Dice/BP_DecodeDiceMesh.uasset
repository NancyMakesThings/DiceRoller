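; Lookup Blueprint that picks the static mesh for a die in the dice roller from its mesh style and die type.
; DecodeDiceMesh switches on style (Round, Sharp, Smooth, or Basic as the default), then on type from D4 to D100, and returns the mesh.
; D100 reuses D10 meshes, and Sharp uses the Basic meshes for D8 and D10, though its D100 gets the Sharp D10 mesh.
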(event EventBeginPlay)

(event EventTick
  (params (DeltaSeconds :type Float%20%28single-precision%29)))

(fn DecodeDiceMesh
  (params (MeshStyle :type MeshStyle%20Enum :default "Default") (DiceType :type DiceType%20Enum :default "D4"))
  (switch Utilities|FlowControl|Switch|SwitchonMeshStyle MeshStyle
    (:Default
      (switch Utilities|FlowControl|Switch|SwitchonDiceType DiceType
        (:D4
          (LocalVariables|SetMesh "/Game/DiceRoller/Core/Dice/Mesh/Basic/SM_D004Basic.SM_D004Basic"))
        (:D6
          (LocalVariables|SetMesh "/Game/DiceRoller/Core/Dice/Mesh/Basic/SM_D006Basic.SM_D006Basic"))
        (:D8
          (LocalVariables|SetMesh "/Game/DiceRoller/Core/Dice/Mesh/Basic/SM_D008Basic.SM_D008Basic"))
        (:D10
          (LocalVariables|SetMesh "/Game/DiceRoller/Core/Dice/Mesh/Basic/SM_D010Basic.SM_D010Basic"))
        (:D12
          (LocalVariables|SetMesh "/Game/DiceRoller/Core/Dice/Mesh/Basic/SM_D012Basic.SM_D012Basic"))
        (:D20
          (LocalVariables|SetMesh "/Game/DiceRoller/Core/Dice/Mesh/Basic/SM_D020_Basic.SM_D020_Basic"))
        (:D100
          (LocalVariables|SetMesh "/Game/DiceRoller/Core/Dice/Mesh/Basic/SM_D010Basic.SM_D010Basic"))))
    (:Round
      (switch Utilities|FlowControl|Switch|SwitchonDiceType DiceType
        (:D4
          (LocalVariables|SetMesh "/Game/DiceRoller/Core/Dice/Mesh/Round/SM_D004Round.SM_D004Round"))
        (:D6
          (LocalVariables|SetMesh "/Game/DiceRoller/Core/Dice/Mesh/Round/SM_D006Round.SM_D006Round"))
        (:D8
          (LocalVariables|SetMesh "/Game/DiceRoller/Core/Dice/Mesh/Round/SM_D008Round.SM_D008Round"))
        (:D10
          (LocalVariables|SetMesh "/Game/DiceRoller/Core/Dice/Mesh/Round/SM_D010Round.SM_D010Round"))
        (:D12
          (LocalVariables|SetMesh "/Game/DiceRoller/Core/Dice/Mesh/Round/SM_D012Round.SM_D012Round"))
        (:D20
          (LocalVariables|SetMesh "/Game/DiceRoller/Core/Dice/Mesh/Round/SM_D020Round.SM_D020Round"))
        (:D100
          (LocalVariables|SetMesh "/Game/DiceRoller/Core/Dice/Mesh/Round/SM_D010Round.SM_D010Round"))))
    (:Sharp
      (switch Utilities|FlowControl|Switch|SwitchonDiceType DiceType
        (:D4
          (LocalVariables|SetMesh "/Game/DiceRoller/Core/Dice/Mesh/Sharp/SM_D004Sharp.SM_D004Sharp"))
        (:D6
          (LocalVariables|SetMesh "/Game/DiceRoller/Core/Dice/Mesh/Sharp/SM_D006Sharp.SM_D006Sharp"))
        (:D8
          (LocalVariables|SetMesh "/Game/DiceRoller/Core/Dice/Mesh/Basic/SM_D008Basic.SM_D008Basic"))
        (:D10
          (LocalVariables|SetMesh "/Game/DiceRoller/Core/Dice/Mesh/Basic/SM_D010Basic.SM_D010Basic"))
        (:D12
          (LocalVariables|SetMesh "/Game/DiceRoller/Core/Dice/Mesh/Sharp/SM_D012Sharp.SM_D012Sharp"))
        (:D20
          (LocalVariables|SetMesh "/Game/DiceRoller/Core/Dice/Mesh/Sharp/SM_D020Sharp.SM_D020Sharp"))
        (:D100
          (LocalVariables|SetMesh "/Game/DiceRoller/Core/Dice/Mesh/Sharp/SM_D010Sharp.SM_D010Sharp"))))
    (:Smooth
      (switch Utilities|FlowControl|Switch|SwitchonDiceType DiceType
        (:D4
          (LocalVariables|SetMesh "/Game/DiceRoller/Core/Dice/Mesh/Smooth/SM_D004Smooth.SM_D004Smooth"))
        (:D6
          (LocalVariables|SetMesh "/Game/DiceRoller/Core/Dice/Mesh/Smooth/SM_D006Smooth.SM_D006Smooth"))
        (:D8
          (LocalVariables|SetMesh "/Game/DiceRoller/Core/Dice/Mesh/Smooth/SM_D008Smooth.SM_D008Smooth"))
        (:D10
          (LocalVariables|SetMesh "/Game/DiceRoller/Core/Dice/Mesh/Smooth/SM_D010Smooth.SM_D010Smooth"))
        (:D12
          (LocalVariables|SetMesh "/Game/DiceRoller/Core/Dice/Mesh/Smooth/SM_D012Smooth.SM_D012Smooth"))
        (:D20
          (LocalVariables|SetMesh "/Game/DiceRoller/Core/Dice/Mesh/Smooth/SM_D020Smooth.SM_D020Smooth"))
        (:D100
          (LocalVariables|SetMesh "/Game/DiceRoller/Core/Dice/Mesh/Smooth/SM_D010Smooth.SM_D010Smooth")))))
  (return (LocalVariables|GetMesh)))